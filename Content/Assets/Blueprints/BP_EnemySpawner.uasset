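; BP_EnemySpawner is a placed spawner actor that creates an enemy pawn at its own transform when play begins.
; BeginPlay switches on EnemyType, and its only handled case spawns a BP_SpiderPawn with AI, ignoring collision failure.
; The Construction Script yaws the spawner toward the first BP_PowerCrystal in the level, so spawned enemies start out facing the crystal.
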(event EventBeginPlay
  (bind _returnvalue (Transformation|GetActorTransform))
  (switch int (Variables|Default|GetEnemyType)
    (:0
      (AI|SpawnAIFromClass "/Game/Assets/Blueprints/BP_SpiderPawn.BP_SpiderPawn_C" 0 (.location _returnvalue) (.rotation _returnvalue) true))))

(event Collision|EventActorBeginOverlap
  (params (OtherActor :type Actor%20Object%20Reference)))

(event EventTick
  (params (DeltaSeconds :type Float%20%28single-precision%29)))

(fn ConstructionScript
  (bind _outactors (Actor|GetAllActorsOfClass "/Game/Assets/Blueprints/BP_PowerCrystal.BP_PowerCrystal_C"))
  (Transformation|SetActorRotation (Math|Rotator|MakeRotator 0.0 0.0 (.yaw (Math|Rotator|FindLookatRotation (Transformation|GetActorLocation) (Transformation|GetActorLocation (Utilities|Array|Get(acopy) _outactors)))))))