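; Spider pawn that attacks power crystals and the top-down player character, and can be destroyed by damage.
; Overlapping either target starts a looping "Attack" timer that applies base damage to the overlap event's last actor; nothing here clears the timer.
; Incoming damage lowers health; at zero or below the mesh turns charred, an explosion effect spawns and the pawn is destroyed.
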(event Custom|Attack
  (Game|Damage|ApplyDamage (stale Collision|EventActorBeginOverlap OtherActor) (Variables|PrimaryAttributes|GetBaseDamage) 0 0))

(event EventBeginPlay)

(event Collision|EventActorBeginOverlap
  (params (OtherActor :type Actor%20Object%20Reference))
  (Utilities|Casting|CastToBP_PowerCrystal OtherActor
    (:then
      _)
    (:CastFailed
      (Utilities|Casting|CastToBP_TopDownCharacter OtherActor)))
  (Utilities|Time|SetTimerbyFunctionName 0 "Attack" 1.0 true))

(event Game|Damage|EventAnyDamage
  (params (Damage :type Float%20%28single-precision%29) (DamageType :type Damage%20Type%20Object%20Reference) (InstigatedBy :type Controller%20Object%20Reference) (DamageCauser :type Actor%20Object%20Reference))
  (if (> (Variables|PrimaryAttributes|GetHealth) 0.0)
    (bind _output_get (Variables|PrimaryAttributes|SetHealth (- (Variables|PrimaryAttributes|GetHealth) Damage)))
    (if (<= _output_get 0.0)
      (Rendering|Material|SetMaterial (Variables|Character|GetMesh) 0 "/Game/Assets/Materials/BaseMetal_Charred.BaseMetal_Charred")
      (Game|SpawnActorfromClass "/Game/StockAssets/StarterContent/Blueprints/Blueprint_Effect_Explosion.Blueprint_Effect_Explosion_C" (Math|Transform|MakeTransform (Transformation|GetActorLocation) "0, 0, 0" "1,1,1") "Undefined" 0 0)
      (Actor|DestroyActor))))

(event EventTick
  (params (DeltaSeconds :type Float%20%28single-precision%29)))

(fn ConstructionScript)