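; Behavior tree task that moves the spider AI's controlled pawn toward the actor stored in a blackboard Target key.
; On execute it uses a cached BP_SpiderController, casting it from the owner actor and storing it when none is set.
; An AIMoveTo toward the target then finishes the task as succeeded with a debug print, or as failed.
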(event EventReceiveExecute
  (params (OwnerActor :type Actor%20Object%20Reference))
  (if (!= (Variables|Default|GetAIController) 0)
    _
    (else
      (bind _asbp_spider_controller (Utilities|Casting|CastToBP_SpiderController OwnerActor))
      (Variables|Default|SetAIController _asbp_spider_controller)))
  (AI|AIMoveTo (Pawn|GetControlledPawn (Variables|Default|GetAIController)) "0, 0, 0" (AI|BehaviorTree|GetBlackboardValueasActor (Variables|Default|GetTarget)) 5.0 false
    (:OnSuccess
      (Development|PrintString "Completed Sucessfully!!" true true "(R=0.000000,G=1.000000,B=0.000000,A=1.000000)")
      (AI|BehaviorTree|FinishExecute true))
    (:OnFail
      (AI|BehaviorTree|FinishExecute false))))