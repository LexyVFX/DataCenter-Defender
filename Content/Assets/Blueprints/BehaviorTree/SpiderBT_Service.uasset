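; Behavior tree service that picks the nearest power crystal or top-down character as the spider AI's target.
; Each tick it caches the spider controller, gathers both actor classes into AvailableTargets and measures their distance from the controlled pawn.
; The closest entry's actor and location go to the Target and TargetLocation blackboard keys, and Target is cleared if none exists.
; Both target and distance arrays persist across ticks without being emptied.
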(event EventTick
  (params (OwnerActor :type Actor%20Object%20Reference) (DeltaSeconds :type Float%20%28single-precision%29))
  (bind _availabletargets (Variables|Default|GetAvailableTargets))
  (bind _targetdistances (Variables|Default|GetTargetDistances))
  (bind _indexofminvalue (Math|Float|MinOfFloatArray _targetdistances))
  (bind _output (Utilities|Array|Get(acopy) _availabletargets _indexofminvalue))
  (Utilities|FlowControl|Sequence
    (:then_0
      (if (!= (Variables|Default|GetAIController) 0)
        _
        (else
          (bind _asbp_spider_controller (Utilities|Casting|CastToBP_SpiderController OwnerActor))
          (Variables|Default|SetAIController _asbp_spider_controller)))
      (bind _outactors (Actor|GetAllActorsOfClass "/Game/Assets/Blueprints/BP_PowerCrystal.BP_PowerCrystal_C"))
      (for _array_element _outactors
        (Utilities|Array|AddUnique (Variables|Default|GetAvailableTargets) _array_element))
      (bind _outactors_2 (Actor|GetAllActorsOfClass "/Game/Assets/Blueprints/BP_TopDownCharacter.BP_TopDownCharacter_C"))
      (for _array_element_2 _outactors_2
        (Utilities|Array|AddUnique (Variables|Default|GetAvailableTargets) _array_element_2)))
    (:then_1
      (for _array_element_3 (Variables|Default|GetAvailableTargets)
        (Utilities|Array|Add (Variables|Default|GetTargetDistances) (Transformation|GetDistanceTo (Pawn|GetControlledPawn (Variables|Default|GetAIController)) _array_element_3)))
      (if (!= _indexofminvalue -1)
        (AI|BehaviorTree|SetBlackboardValueasVector (Variables|Default|GetTargetLocation) (Transformation|GetActorLocation _output))
        (Class|BTFunctionLibrary|SetBlackboardValueasObject (Variables|Default|GetTarget) _output)
        (else
          (Class|BTFunctionLibrary|SetBlackboardValueasObject (Variables|Default|GetTarget)))))))