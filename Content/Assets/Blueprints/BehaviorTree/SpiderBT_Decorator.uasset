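; Behavior tree decorator for the spider AI that tests whether its target is at or beyond targeting range.
; It casts the owner to BP_SpiderController, then measures the distance between the controlled pawn and the actor in the Target blackboard key.
; The condition passes when that distance is greater than or equal to TargetingRange.
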(fn PerformConditionCheck
  (params (OwnerActor :type Actor%20Object%20Reference))
  (bind _asbp_spider_controller (Utilities|Casting|CastToBP_SpiderController OwnerActor))
  (Variables|Default|SetAIController _asbp_spider_controller)
  (return (>= (Math|Vector|VectorLength (- (Transformation|GetActorLocation (AI|BehaviorTree|GetBlackboardValueasActor (Variables|Default|GetTarget))) (Transformation|GetActorLocation (Pawn|GetControlledPawn (Variables|Default|GetAIController))))) (Variables|Default|GetTargetingRange))))