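; AI controller for a spider pawn that walks it toward the first BP_PowerCrystal in the level.
; BeginPlay starts a looping timer that re-issues an AI MoveTo to the crystal, cleared when a move succeeds or fails.
; A similar player-chasing event exists, but its timer is disconnected.
; Behavior tree startup and eased timeline rotation toward the crystal are also unwired, and OnPossess is empty.
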(event Custom|Track%20Power%20Core
  (bind _outactors (Actor|GetAllActorsOfClass "/Game/Assets/Blueprints/BP_PowerCrystal.BP_PowerCrystal_C"))
  (AI|AIMoveTo (Pawn|GetControlledPawn) "0, 0, 0" (Utilities|Array|Get(acopy) _outactors) 2e+02 false
    (:OnSuccess
      _)
    (:OnFail
      _))
  (Utilities|Time|ClearTimerbyFunctionName 0 "Track Power Core"))

(event Custom|Track%20Player
  (AI|AIMoveTo (Pawn|GetControlledPawn) "0, 0, 0" (Game|GetPlayerCharacter 0) 1e+02 false
    (:OnSuccess
      (Development|PrintString "Completed Sucessfully!!" true true "(R=0.000000,G=1.000000,B=0.000000,A=1.000000)"))
    (:OnFail
      (Development|PrintString "Failed" true true "(R=0.800000,G=0.000000,B=0.000000,A=1.000000)")))
  (Utilities|Time|ClearTimerbyFunctionName 0 "Track Player"))

(event EventBeginPlay
  (Utilities|Time|SetTimerbyFunctionName 0 "Track Power Core" 1.0 true))

(event EventTick
  (params (DeltaSeconds :type Float%20%28single-precision%29)))

(event EventOnPossess
  (params (PossessedPawn :type Pawn%20Object%20Reference)))

(fn ConstructionScript)