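; BP_PowerCrystal is a destructible crystal whose destruction loses the game.
; Tick spins its mesh parts while alive and blends the crystal's emissive color by remaining health ratio.
; AnyDamage drains health; a hit after depletion triggers a one-time explosion and lethal damage to every Pawn.
; The death sequence also enables physics on the parts, swaps in charred materials, prints a lose message and reloads OverWorld after a delay.
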(event EventBeginPlay)

(event Collision|EventActorBeginOverlap
  (params (OtherActor :type Actor%20Object%20Reference)))

(event Game|Damage|EventAnyDamage
  (params (Damage :type Float%20%28single-precision%29) (DamageType :type Damage%20Type%20Object%20Reference) (InstigatedBy :type Controller%20Object%20Reference) (DamageCauser :type Actor%20Object%20Reference))
  (bind _returnvalue (Transformation|GetActorTransform))
  (if (> (Variables|PrimaryAttributes|GetHealth) 0.0)
    (Variables|PrimaryAttributes|SetHealth (- (Variables|PrimaryAttributes|GetHealth) Damage))
    (elif (Variables|Default|GetbAlive)
      (Utilities|FlowControl|DoOnce false
        (:Completed
          (Game|SpawnActorfromClass "/Game/StockAssets/StarterContent/Blueprints/Blueprint_Effect_Explosion.Blueprint_Effect_Explosion_C" (Math|Transform|MakeTransform (Math|Vector|MakeVector (.x (.location _returnvalue)) (.y (.location _returnvalue)) (+ (.z (.location _returnvalue)) 4.2e+02)) "0, 0, 0" "15.000000,15.000000,15.000000") "Undefined" 0 0)
          (Variables|Default|SetbAlive false)
          (bind _outactors (Actor|GetAllActorsOfClass "/Script/Engine.Pawn"))
          (for _array_element _outactors
            (Game|Damage|ApplyDamage _array_element 99999.0 0 0)
            (Physics|SetSimulatePhysics (Variables|Default|GetServer_Crystal_Tube001) true)
            (Rendering|Material|SetMaterial (Variables|Default|GetServer_Crystal_Object) 0 "/Game/Assets/Materials/BaseMetal_Charred.BaseMetal_Charred")
            (Rendering|Material|SetMaterial (Variables|Default|GetServer_Crystal_Cylinder001) 0 "/Game/Assets/Materials/DeadCrystal.DeadCrystal")
            (Development|PrintString "You Lose!! Try Again!" true true "(R=0.800000,G=0.000000,B=0.000000,A=1.000000)")
            (Utilities|FlowControl|Delay 8.0)
            (Game|OpenLevel(byName) "OverWorld")))))))

(event EventTick
  (params (DeltaSeconds :type Float%20%28single-precision%29))
  (Utilities|FlowControl|Sequence
    (:then_0
      (Rendering|Material|SetVectorParameterValueonMaterials (Variables|Default|GetServer_Crystal_Cylinder001) "EmColor" (Math|Interpolation|Ease "Linear" (/ (Variables|PrimaryAttributes|GetHealth) (Variables|PrimaryAttributes|GetMaxHealth)) (Math|Conversions|ToVector(LinearColor) (Variables|PrimaryAttributes|GetCrystalEndColor)) (Math|Conversions|ToVector(LinearColor) (Variables|PrimaryAttributes|GetCrystalBaseColor)))))
    (:then_1
      (if (Variables|Default|GetbAlive)
        (Utilities|FlowControl|Sequence
          (:then_0
            (Transformation|AddLocalRotation (Variables|Default|GetServer_Crystal_Cylinder001) (Math|Rotator|MakeRotator 0.0 0.0 (* DeltaSeconds 15.0)) false false))
          (:then_1
            (Transformation|AddLocalRotation (Variables|Default|GetServer_Crystal_Tube001) (Math|Rotator|MakeRotator 0.0 0.0 (* DeltaSeconds -15.0)) false false))
          (:then_2
            (Transformation|AddLocalRotation (Variables|Default|GetServer_Crystal_Object) (Math|Rotator|MakeRotator 0.0 0.0 (* DeltaSeconds 1e+01)) false false))
          (:then_3
            (Transformation|AddLocalRotation (Variables|Default|GetServer_Crystal_Object002) (Math|Rotator|MakeRotator 0.0 0.0 (* DeltaSeconds 8.0)) false false)))))))

(fn ConstructionScript)