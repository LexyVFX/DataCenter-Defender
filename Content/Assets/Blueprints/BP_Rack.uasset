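; BP_Rack is an interactable rack with a boolean Status shown by its StatusLight, green when true and red when false.
; Overlap by the FirstPersonCharacter prints an interact prompt, and the Interact event opens the level NewMap only while Status is false.
; StatusToggle flips Status and recolors the light, while the construction script sets the initial color from the current value.
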(event Custom|Interact
  (if (not (Variables|Default|GetbStatus))
    (Game|OpenLevel(byName) "NewMap")))

(event Custom|StatusToggle
  (bind _status_light (Variables|Default|GetStatus%20light))
  (if (Variables|Default|GetbStatus)
    (Variables|Default|SetbStatus false)
    (Rendering|Components|Light|SetLightColor _status_light "(R=1.000000,G=0.000000,B=0.000000,A=1.000000)" true)
    (else
      (Variables|Default|SetbStatus true)
      (Rendering|Components|Light|SetLightColor _status_light "(R=0.000000,G=1.000000,B=0.000000,A=1.000000)" true))))

(event EventBeginPlay)

(event Collision|EventActorBeginOverlap
  (params (OtherActor :type Actor%20Object%20Reference))
  (Utilities|Casting|CastToFirstPersonCharacter OtherActor)
  (Development|PrintString "Press F to Interact" true true "(R=0.000000,G=1.000000,B=0.000000,A=1.000000)"))

(event EventTick
  (params (DeltaSeconds :type Float%20%28single-precision%29)))

(fn ConstructionScript
  (bind _status_light (Variables|Default|GetStatus%20light))
  (if (Variables|Default|GetbStatus)
    (Rendering|Components|Light|SetLightColor _status_light "(R=0.000000,G=1.000000,B=0.000000,A=1.000000)" true)
    (else
      (Rendering|Components|Light|SetLightColor _status_light "(R=1.000000,G=0.000000,B=0.000000,A=1.000000)" true))))